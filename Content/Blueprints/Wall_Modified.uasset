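; Wall_Modified is a Blueprint for a wall that switches between two brick materials when touched.
; A touch-begin event on the Wall component drives a FlipFlop that alternately sets material slot 0 to the new clay brick and beveled clay brick materials.
; The construction script stores a dynamic material instance of that slot in DynamicWallVariable, but the touch logic does not use it.
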(event OnInputTouchBegin(Wall)
  (params (FingerIndex :type ETouchIndex%20Enum :default "Touch1") (TouchedComponent :type Primitive%20Component%20Object%20Reference))
  (Utilities|FlowControl|FlipFlop
    (:A
      (Rendering|Material|SetMaterial (Variables|Default|GetWall) 0 "/Game/MobileStarterContent/Materials/M_Brick_Clay_New.M_Brick_Clay_New"))
    (:B
      (Rendering|Material|SetMaterial (Variables|Default|GetWall) 0 "/Game/MobileStarterContent/Materials/M_Brick_Clay_Beveled.M_Brick_Clay_Beveled"))))

(event EventBeginPlay)

(event EventActorBeginOverlap
  (params (OtherActor :type Actor%20Object%20Reference)))

(event EventTick
  (params (DeltaSeconds :type Float%20%28single-precision%29)))

(fn ConstructionScript
  (bind _returnvalue (Rendering|Material|CreateDynamicMaterialInstance (Variables|Default|GetWall) 0 0 :!class /Script/Engine.PrimitiveComponent))
  (Variables|Default|SetDynamic%20Wall%20Variable _returnvalue))