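; ConferenceWall is a touch-reactive wall Blueprint that swaps the surface material of its mesh.
; Each touch begin on the wall runs a FlipFlop that alternates element 0 between pine wood and polished walnut floor materials.
; The construction script creates and stores a dynamic material instance for that element, but the touch logic sets the material assets directly and never uses it.
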(event OnInputTouchBegin(ConferenceWall)
  (params (FingerIndex :type ETouchIndex%20Enum :default "Touch1") (TouchedComponent :type Primitive%20Component%20Object%20Reference))
  (Utilities|FlowControl|FlipFlop
    (:A
      (Rendering|Material|SetMaterial (Variables|Default|GetConferenceWall) 0 "/Game/MobileStarterContent/Materials/M_Wood_Pine.M_Wood_Pine"))
    (:B
      (Rendering|Material|SetMaterial (Variables|Default|GetConferenceWall) 0 "/Game/MobileStarterContent/Materials/M_Wood_Floor_Walnut_Polished.M_Wood_Floor_Walnut_Polished"))))

(event EventBeginPlay)

(event Collision|EventActorBeginOverlap
  (params (OtherActor :type Actor%20Object%20Reference)))

(event EventTick
  (params (DeltaSeconds :type Float%20%28single-precision%29)))

(fn ConstructionScript
  (bind _returnvalue (Rendering|Material|CreateDynamicMaterialInstance (Variables|Default|GetConferenceWall) 0 0 :!class /Script/Engine.PrimitiveComponent))
  (Variables|Default|SetDynamic%20Wall%20Variable _returnvalue))